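; Interactor component for the BP_Assasin character that tracks the current BP_Interactuable it can interact with.
; It binds overlap events on the owner's single shape tagged InteractorShape, keeping the closer interactable whenever a new overlap begins.
; Selection updates the owner's prompt text; ending overlap with the active one clears it without reselecting.
; Getters expose the selected interactable's actor, action and transform.
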(event Custom|OnComponentBeginOverlap_Event
  (params (OverlappedComponent :type Primitive%20Component%20Object%20Reference) (OtherActor :type Actor%20Object%20Reference) (OtherComp :type Primitive%20Component%20Object%20Reference) (OtherBodyIndex :type Integer) (bFromSweep :type Boolean) (SweepResult :type Hit%20Result%20Structure%20%28by%20ref%29))
  ;[1 1 1] Empiezo overlap
  (CallFunction|BeginOverlap OtherActor))

(event Custom|OnComponentEndOverlapEvent
  (params (OverlappedComponent :type Primitive%20Component%20Object%20Reference) (OtherActor :type Actor%20Object%20Reference) (OtherComp :type Primitive%20Component%20Object%20Reference) (OtherBodyIndex :type Integer))
  ;[1 1 1] Termino overlap
  (CallFunction|EndOverlap OtherActor))

(event EventBeginPlay
  (bind _returnvalue (Components|GetOwner))
  (bind _returnvalue_2 (Actor|GetComponentsbyTag _returnvalue "/Script/Engine.ShapeComponent" "InteractorShape"))
  ;[1 1 1] Me guardo quien es el thridPersonOwner, que sé que ejecuta la interfaz
  (bind _asbp_assasin (Utilities|Casting|CastToBP_Assasin (Components|GetOwner))
    (:then
      (Variables|Default|SetTPOwner _asbp_assasin)
      (if (== (Utilities|Array|Length _returnvalue_2) 1)
        ;[1 1 1] Esta es mi shape
        (bind _output_get (Variables|Default|SetInteractorShape (Utilities|Array|Get(acopy) _returnvalue_2)))
        (Collision|BindEventtoOnComponentBeginOverlap _output_get (delegate Custom|OnComponentBeginOverlap_Event))
        (Collision|BindEventtoOnComponentEndOverlap _output_get (delegate Custom|OnComponentEndOverlapEvent))
        (else
          (Development|PrintString "Error de inicialización. 0 o más de una InteractorShapes en este actor")
          (Components|Tick|SetComponentTickEnabled false))))
    (:CastFailed
      (Development|PrintString "NotThridPersonCharacter"))))

(event EventTick
  (params (DeltaSeconds :type Float%20%28single-precision%29)))

(fn BeginOverlap
  (params (OverlapActor :type Actor%20Object%20Reference))
  (bind _returnvalue (Actor|GetComponentbyClass OverlapActor "/Game/Blueprints/Interactor/BP_Interactuable.BP_Interactuable_C"))
  ;[1 1 1] No hay overlap conmigo mismo
  (Development|PrintString "Overlapping")
  (if (== OverlapActor (Variables|Default|GetTPOwner))
    (Development|PrintString "OverlappingWithMyself")
    (else
      (Development|PrintString "OverlapingWithCar")
      ;[1 1 1] We can get more than one component, here we assume there is only one
      (Utilities|IsValid _returnvalue
        (:Is%20Valid
          (Development|PrintString "NowIsValid")
          (bind _choosen (CallFunction|SelectInteractuable _returnvalue))
          ;;[1 1 1] Decirle el texto a mostrar que se actualice
          (Default|UpdateInteractuableText (Variables|Default|GetTPOwner) (Variables|/Game/Blueprints/Interactor/BP_Interactuable.BP_Interactuable_C|GetTextToShow _choosen)))
        (:Is%20Not%20Valid
          (Development|PrintString "MissingInteractuableComponent"))))))

(fn EndOverlap
  (params (Actor :type Actor%20Object%20Reference))
  ;[1 1 1] Cogemos el actor con el que hemos terminado de hacer overlap, buscamos el componente interactuable, y si es el que teníamos como activo llamamos a la función de limpieza
  (if (== (Variables|Default|GetInteractuableComponent) (Actor|GetComponentbyClass Actor "/Game/Blueprints/Interactor/BP_Interactuable.BP_Interactuable_C"))
    (Default|CleanInteractuable (Variables|Default|GetTPOwner))
    (Variables|Default|SetInteractuableComponent 0)
    (Default|UpdateInteractuableText (Variables|Default|GetTPOwner) "   ")
    (else
      (Development|PrintString "CantGetInteractuable"))))

(fn GetInteractuableActor
  ;[1 1 1] Me devuelve el actor en el que encontramos el componente
  (bind _interactuablecomponent (Variables|Default|GetInteractuableComponent)
    (:then
      (return (Components|GetOwner _interactuablecomponent) true))
    (:else
      (return 0 false))))

(fn SelectInteractuable
  (params (NewInteractuable :type BP%20Interactuable%20Object%20Reference))
  (bind _returnvalue (Components|GetOwner))
  (bind _returnvalue_2 (Transformation|GetActorLocation _returnvalue))
  (Utilities|IsValid (Variables|Default|GetInteractuableComponent)
    (:Is%20Valid
      ;[1 1 1] Comprobamos cual de los dos es, el que está más cerca o si nos hemos acercado demasiado al siguiente
      (if (< (Math|Vector|Distance(Vector) _returnvalue_2 (Transformation|GetWorldLocation NewInteractuable)) (Math|Vector|Distance(Vector) _returnvalue_2 (Transformation|GetWorldLocation (Variables|Default|GetInteractuableComponent))))
        (bind _output_get (Variables|Default|SetInteractuableComponent NewInteractuable))
        (return _output_get)
        (else
          (return (Variables|Default|GetInteractuableComponent)))))
    (:Is%20Not%20Valid
      (Development|PrintString "SlectNotValid")
      ;[1 1 1] Si no hay nada seteado seteamos el nuevo interactuable
      (bind _output_get_2 (Variables|Default|SetInteractuableComponent NewInteractuable))
      (return _output_get_2))))

(fn HasInteractuable
  ;[1 1 1] Me decuelve si es interactuable
  (bind _interactuablecomponent (Variables|Default|GetInteractuableComponent)
    (:then
      (return true _interactuablecomponent))
    (:else
      (return false 0))))

(fn GetInteractuableAction
  ;[1 1 1] Devuelve la acción seteada si existe alguna
  (bind _interactuablecomponent (Variables|Default|GetInteractuableComponent)
    (:then
      (return (Variables|/Game/Blueprints/Interactor/BP_Interactuable.BP_Interactuable_C|GetActionToPlay _interactuablecomponent)))
    (:else
      (return 0))))

(fn GetInteractuablePosition
  ;[1 1 1] Devuelve la posición si existe algún interactuable
  (bind _interactuablecomponent (Variables|Default|GetInteractuableComponent)
    (:then
      (return (Transformation|GetWorldTransform _interactuablecomponent)))
    (:else
      ;[1 1 1] Si no, devuelve la posición de nuestro propio actor
      (return (Transformation|GetActorTransform (Variables|Default|GetTPOwner))))))