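; BP_SensorBar is a sensor bar actor that detects the player on contact to sound an alarm.
; Overlaps on its Trigger component pass the other actor to DetectPlayer, which is defined outside this file.
; Interact toggles the Activated state, switching actor collision and the visibility of BarsParent and its children on or off together.
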(event OnComponentBeginOverlap(Trigger)
  (params (OverlappedComponent :type Primitive%20Component%20Object%20Reference) (OtherActor :type Actor%20Object%20Reference) (OtherComp :type Primitive%20Component%20Object%20Reference) (OtherBodyIndex :type Integer) (bFromSweep :type Boolean) (SweepResult :type Hit%20Result%20Structure%20%28by%20ref%29))
  ;[1 1 1] Cuando te toca el player suena la alarma
  (CallFunction|DetectPlayer OtherActor))

(event EventBeginPlay)

(event Collision|EventActorBeginOverlap
  (params (OtherActor :type Actor%20Object%20Reference)))

(event EventTick
  (params (DeltaSeconds :type Float%20%28single-precision%29)))

(event EventInteract
  ;[1 1 1] Colisión del sensor
  (if (not (Variables|Default|GetActivated))
    (Collision|SetActorEnableCollision true)
    (Rendering|SetVisibility (Variables|Default|GetBarsParent) true true)
    (Variables|Default|SetActivated true)
    (else
      (Collision|SetActorEnableCollision false)
      (Rendering|SetVisibility (Variables|Default|GetBarsParent) false true)
      (Variables|Default|SetActivated false))))

(fn ConstructionScript
  (|CallParentFunction))