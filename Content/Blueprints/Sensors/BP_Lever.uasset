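; BP_Lever is an interactable lever that triggers a linked OutputActor.
; Each interaction plays an attenuated sound, then sends InteractMessage through BPI_Interact if the output is valid and implements that interface.
; Only in that case does it toggle Activated and play or reverse a timeline that rotates the lever mesh between two poses.
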(event Custom|SwitchLevel
  ;[1 1 1] Girar palanca
  (Audio|PlaySoundatLocation "/Engine/VREditor/Sounds/UI/Floating_UI_Close-002.Floating_UI_Close-002" (Transformation|GetActorLocation) "0, 0, 0" 1.0 1.0 0.0 "/Game/Audio/Alarm/SA_Sensor.SA_Sensor" 0 0 0)
  (bind _outputactor (Variables|Default|GetOutputActor)
    (:then
      (if (Utilities|DoesObjectImplementInterface _outputactor "/Game/Blueprints/Interfaces/BPI_Interact.BPI_Interact_C")
        (Class|BPIInteract|Interact(Message) _outputactor)
        (if (not (Variables|Default|GetActivated))
          (Variables|Default|SetActivated true)
          (bind _rotation (Timeline|PullLeverTimeLine Play)
            (:Update
              (Transformation|SetRelativeRotation (Variables|Default|GetLever) (Math|Rotator|Lerp(Rotator) "120.000000,0.000000,0.000000" "50.000000,0.000000,0.000000" _rotation) false false)))
          (else
            (Variables|Default|SetActivated false)
            (Timeline|PullLeverTimeLine Reverse)))))
    (:else)))

(event EventInteract
  (CallFunction|SwitchLevel))

(fn ConstructionScript)