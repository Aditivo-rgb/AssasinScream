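; Rotating sensor that detects the player inside its trigger zone and raises detection once they linger too long.
; A Motion timeline sweeps the head back and forth, using a FlipFlop to alternate reverse and play.
; On overlap, a fast looping timer fills the player's detection meter until it calls DetectPlayer and marks the widget detected.
; Leaving the zone stops the timer and resets the count, clearing the meter unless already detected.
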(event OnComponentBeginOverlap(TriggerDetectionZone)
  (params (OverlappedComponent :type Primitive%20Component%20Object%20Reference) (OtherActor :type Actor%20Object%20Reference) (OtherComp :type Primitive%20Component%20Object%20Reference) (OtherBodyIndex :type Integer) (bFromSweep :type Boolean) (SweepResult :type Hit%20Result%20Structure%20%28by%20ref%29))
  ;[0 0 0] Cuando te toca el player suena la alarma
  ;;[1 1 1] Es el player
  (if (Actor|ActorHasTag OtherActor "Player")
    (Variables|Default|SetPlayerInZone true)
    ;;[1 1 1] Empiezo a contar
    (bind _returnvalue (Utilities|Time|SetTimerbyEvent (delegate Custom|Count) 0.002 true))
    (Variables|Default|SetCountTimer _returnvalue)))

(event OnComponentEndOverlap(TriggerDetectionZone)
  (params (OverlappedComponent :type Primitive%20Component%20Object%20Reference) (OtherActor :type Actor%20Object%20Reference) (OtherComp :type Primitive%20Component%20Object%20Reference) (OtherBodyIndex :type Integer))
  (bind _player (Variables|Default|GetPlayer))
  (bind _detectedmeterwidget (Variables|/Game/Blueprints/Player/BP_Assasin.BP_Assasin_C|GetDetectedmeterWidget _player))
  ;[1 1 1] Quitar cuando sale la barra
  (if (Actor|ActorHasTag OtherActor "Player")
    (Variables|Default|SetPlayerInZone false)
    (Utilities|Time|ClearandInvalidateTimerbyHandle (Variables|Default|GetCountTimer))
    (Variables|Default|SetTimeUnderZone 0.0)
    (if (not (Variables|/Game/UI/WBP_Detection.WBP_Detection_C|GetIsDetected _detectedmeterwidget))
      (Progress|SetPercent (Variables|/Game/UI/WBP_Detection.WBP_Detection_C|GetProgressBar _detectedmeterwidget) 0.0))))

(event Custom|Count
  ;[0 0 0] Cuando te toca el player suena la alarma
  ;;[1 1 1] Empiezo a llenar la barra
  (Variables|Default|SetTimeUnderZone (+ (Variables|Default|GetTimeUnderZone) 0.005))
  (CallFunction|UpdateProgressBar)
  (if (>= (Variables|Default|GetTimeUnderZone) (Variables|Default|GetMaxTimeUnderZone))
    ;;[1 1 1] Detecto y doy alarma
    (CallFunction|DetectPlayer (stale OnComponentBeginOverlap(TriggerDetectionZone) OtherActor))
    ;[1 1 1] Paro el timer y pongo el texto
    (Utilities|Time|ClearandInvalidateTimerbyHandle (Variables|Default|GetCountTimer))
    (Default|Detected (Variables|/Game/Blueprints/Player/BP_Assasin.BP_Assasin_C|GetDetectedmeterWidget (Variables|Default|GetPlayer)))))

(event Custom|UpdateProgressBar
  (bind _player (Variables|Default|GetPlayer))
  (bind _detectedmeterwidget (Variables|/Game/Blueprints/Player/BP_Assasin.BP_Assasin_C|GetDetectedmeterWidget _player))
  ;[0 0 0] Cuando te toca el player suena la alarma
  ;;[1 1 1] Porcentaje del widget
  (if (not (Variables|/Game/UI/WBP_Detection.WBP_Detection_C|GetIsDetected _detectedmeterwidget))
    (Progress|SetPercent (Variables|/Game/UI/WBP_Detection.WBP_Detection_C|GetProgressBar _detectedmeterwidget) (/ (Variables|Default|GetTimeUnderZone) (Variables|Default|GetMaxTimeUnderZone)))))

(event EventBeginPlay
  ;[1 1 1] Rotación del sensor
  (Utilities|FlowControl|Sequence
    (:then_0
      (bind _rotation (Timeline|Motion Play)
        (:Update
          (Transformation|SetRelativeRotation (Variables|Default|GetHead) (Math|Rotator|Lerp(Rotator) "0.000000,90.000000,0.000000" "0.000000,-90.000000,0.000000" _rotation) false false))
        (:Finished
          (Utilities|FlowControl|FlipFlop
            (:A
              (Timeline|Motion Reverse))
            (:B
              (Timeline|Motion Play))))))
    (:then_1
      (bind _asbp_assasin (Utilities|Casting|CastToBP_Assasin (Game|GetPlayerCharacter 0)))
      (Variables|Default|SetPlayer _asbp_assasin))))

(fn ConstructionScript
  (|CallParentFunction))