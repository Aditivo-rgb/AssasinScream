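; BP_Alarm is a stealth-game alarm actor that raises a level-wide alert against the player.
; StartAlarm, gated by an active flag, spawns the alarm sound at the actor's location and calls AlertGuards.
; AlertGuards sets HasSeenPlayer on every BP_Guard's AI blackboard, then has GM_StealthGamemode switch the music to chase.
; StopAlarm only silences the sound and clears the flag, leaving guards and music untouched.
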(event Custom|StartAlarm
  ;[1 1 1] Sonido Alarma
  (if (not (Variables|Default|GetAlarmActive))
    (bind _returnvalue (Audio|SpawnSoundatLocation "/Game/Audio/Alarm/MS_Alarm.MS_Alarm" (Transformation|GetActorLocation) "0, 0, 0" 1.0 1.0 0.0 0 0))
    (Variables|Default|SetAlarmSound _returnvalue)
    (Variables|Default|SetAlarmActive true)
    (CallFunction|AlertGuards)))

(event Custom|StopAlarm
  ;[1 1 1] Apagar alarma
  (if (Variables|Default|GetAlarmActive)
    (Audio|Components|Audio|FadeOut (Variables|Default|GetAlarmSound) 0.0 0.0 "Linear" :!class /Script/Engine.AudioComponent)
    (Variables|Default|SetAlarmActive false)))

(event Custom|AlertGuards
  ;[1 1 1] Avisa a todos los guardias
  (bind _outactors (Actor|GetAllActorsOfClass "/Game/AI/BP_Guard.BP_Guard_C"))
  (for _array_element _outactors
    (bind _asbp_ai_guard (Utilities|Casting|CastToBP_AI_Guard (AI|GetAIController _array_element)))
    (AI|Components|Blackboard|SetValueasBool (AI|GetBlackboard _asbp_ai_guard) (Utilities|Name|MakeLiteralName "HasSeenPlayer") true)
    (Development|PrintString "Todos a por el player"))
  ;[1 1 1] Suena la música de persecución
  (bind _asgm_stealth_gamemode (Utilities|Casting|CastToGM_StealthGamemode (Game|GetGameMode)))
  (Default|SwitchMusic _asgm_stealth_gamemode))

(fn ConstructionScript)