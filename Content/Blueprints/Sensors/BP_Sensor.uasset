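; BP_Sensor is a detection sensor that triggers the level's alarm when it spots the player.
; DetectPlayer fires once for an actor tagged Player, latching HasDetected and playing a camera shutter sound at the sensor.
; It then finds BP_Alarm in the level, calls StartAlarm and animates the point light intensity with a timeline like a flash.
; If no alarm exists, it only prints a warning.
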(event Custom|DetectPlayer
  (params (ActorDetected :type Actor%20Object%20Reference))
  ;[1 1 1] Si choca con el player, seteo que lo ha hecho y reproduzco sonido
  (if (and (Actor|ActorHasTag ActorDetected "Player") (not (Variables|Default|GetHasDetected)))
    (Variables|Default|SetHasDetected true)
    (Audio|PlaySoundatLocation "/Engine/VREditor/Sounds/UI/Camera_Shutter.Camera_Shutter" (Transformation|GetActorLocation) "0, 0, 0" 1.0 1.0 0.0 "/Game/Audio/Alarm/SA_Alarm.SA_Alarm" 0 0 0)
    ;[1 1 1] busco la alarma de mi nivel
    (bind _returnvalue (Actor|GetActorOfClass "/Game/Blueprints/Sensors/BP_Alarm.BP_Alarm_C"))
    (Utilities|IsValid _returnvalue
      (:Is%20Valid
        (Default|StartAlarm _returnvalue)
        ;[1 1 1] Emito la luz con animación
        (bind _intensity (Timeline|PointLightTimeline Play)
          (:Update
            (Rendering|Components|Light|SetIntensity (Variables|Default|GetPointLight) (Math|Float|Lerp 0.0 1e+05 _intensity)))))
      (:Is%20Not%20Valid
        (Development|PrintString "No hay alarmas")))))

(fn ConstructionScript)