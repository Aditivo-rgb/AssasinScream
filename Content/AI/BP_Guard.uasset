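; BP_Guard is a guard character that the player can take down.
; An overlap radius shows a takedown prompt widget to Player-tagged actors while the guard is alive.
; TakeDown, gated by CanTakeDown, plays a victim montage, hides the prompt, marks the guard dead and returns a reference location and the guard's rotation.
; A delayed event then enables mesh physics and disables movement for the ragdoll.
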(event OnComponentBeginOverlap(TakeDownRadoius)
  (params (OverlappedComponent :type Primitive%20Component%20Object%20Reference) (OtherActor :type Actor%20Object%20Reference) (OtherComp :type Primitive%20Component%20Object%20Reference) (OtherBodyIndex :type Integer) (bFromSweep :type Boolean) (SweepResult :type Hit%20Result%20Structure%20%28by%20ref%29))
  (if (and (Actor|ActorHasTag OtherActor "Player") (not (Variables|Default|GetDead)))
    (Rendering|SetVisibility (Variables|Default|GetTakeDownWidget) true false)
    (else
      (Development|PrintString "No tag"))))

(event OnComponentEndOverlap(TakeDownRadoius)
  (params (OverlappedComponent :type Primitive%20Component%20Object%20Reference) (OtherActor :type Actor%20Object%20Reference) (OtherComp :type Primitive%20Component%20Object%20Reference) (OtherBodyIndex :type Integer))
  (if (Actor|ActorHasTag OtherActor "Player")
    (Rendering|SetVisibility (Variables|Default|GetTakeDownWidget) false false)
    (else
      (Development|PrintString "No tag"))))

(event Custom|TakeDownRagdoll
  (Utilities|FlowControl|Delay 1.27)
  (Physics|SetSimulatePhysics (Variables|Character|GetMesh) true)
  (Pawn|Components|CharacterMovement|SetMovementMode (Variables|Character|GetCharacterMovement) "MOVE_None" 0))

(event EventBeginPlay)

(event Collision|EventActorBeginOverlap
  (params (OtherActor :type Actor%20Object%20Reference)))

(event EventTick
  (params (DeltaSeconds :type Float%20%28single-precision%29)))

(fn ConstructionScript)

(fn TakeDown
  (if (Variables|Default|GetCanTakeDown)
    (Animation|PlayAnimMontage "/Game/Characters/Assasin/TakeDowns/Takedown_Victim_Montage.Takedown_Victim_Montage" 1.0 "None")
    (CallFunction|TakeDownRagdoll)
    (Rendering|SetVisibility (Variables|Default|GetTakeDownWidget) false false)
    (Variables|Default|SetDead true)
    (return (Transformation|GetWorldLocation (Variables|Default|GetREF)) (Transformation|GetActorRotation) (Variables|Default|GetCanTakeDown) 0)))